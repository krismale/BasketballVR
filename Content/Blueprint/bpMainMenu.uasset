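; VR main menu actor with two 3D buttons, Start Game and Levels, operated with motion controllers.
; Overlap by a BpMotionController swaps a button's material and text color and sets its targeting flag.
; Either Grab input opens the Court1 level while Start Game is targeted; the Levels branch is empty.
; BeginPlay caches the player's MotionControllerPawn, which these graphs never use afterward.
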(event OnComponentBeginOverlap(LevelsBlock)
  (params (OverlappedComponent :type Primitive%20Component%20Object%20Reference) (OtherActor :type Actor%20Object%20Reference) (OtherComp :type Primitive%20Component%20Object%20Reference) (OtherBodyIndex :type Integer) (bFromSweep :type Boolean) (SweepResult :type Hit%20Result%20Structure%20%28by%20ref%29))
  (if (== (Utilities|GetClass OtherActor) "/Game/Blueprint/VirtualRealityBP/bpMotionController.bpMotionController_C")
    (Rendering|Material|SetMaterial (Variables|Default|GetLevelsBlock) 0 "/Game/Meshes/Menu/Materials/highlightedBackground.highlightedBackground")
    (Rendering|Components|TextRender|SetTextRenderColor (Variables|Default|GetLevelsText) (Math|Conversions|ToColor(LinearColor) (Math|Color|MakeColor 255.0 255.0 255.0 255.0)))
    (Variables|Default|SetisTargetingLevels true)))

(event OnComponentEndOverlap(LevelsBlock)
  (params (OverlappedComponent :type Primitive%20Component%20Object%20Reference) (OtherActor :type Actor%20Object%20Reference) (OtherComp :type Primitive%20Component%20Object%20Reference) (OtherBodyIndex :type Integer))
  (if (== (Utilities|GetClass OtherActor) "/Game/Blueprint/VirtualRealityBP/bpMotionController.bpMotionController_C")
    (Rendering|Material|SetMaterial (Variables|Default|GetLevelsBlock) 0 "/Game/Meshes/Menu/Materials/unhighlightedBackground.unhighlightedBackground")
    (Rendering|Components|TextRender|SetTextRenderColor (Variables|Default|GetLevelsText) (Math|Conversions|ToColor(LinearColor) (Math|Color|MakeColor 0.0 0.0 0.0 255.0)))
    (Variables|Default|SetisTargetingLevels false)))

(event OnComponentBeginOverlap(StartLevel1)
  (params (OverlappedComponent :type Primitive%20Component%20Object%20Reference) (OtherActor :type Actor%20Object%20Reference) (OtherComp :type Primitive%20Component%20Object%20Reference) (OtherBodyIndex :type Integer) (bFromSweep :type Boolean) (SweepResult :type Hit%20Result%20Structure%20%28by%20ref%29))
  (if (== (Utilities|GetClass OtherActor) "/Game/Blueprint/VirtualRealityBP/bpMotionController.bpMotionController_C")
    (Rendering|Material|SetMaterial (Variables|Default|GetStartLevel1) 0 "/Game/Meshes/Menu/Materials/highlightedBackground.highlightedBackground")
    (Rendering|Components|TextRender|SetTextRenderColor (Variables|Default|GetStartGameText) (Math|Conversions|ToColor(LinearColor) (Math|Color|MakeColor 255.0 255.0 255.0 255.0)))
    (Variables|Default|SetisTargetingStartLevel1 true)))

(event OnComponentEndOverlap(StartLevel1)
  (params (OverlappedComponent :type Primitive%20Component%20Object%20Reference) (OtherActor :type Actor%20Object%20Reference) (OtherComp :type Primitive%20Component%20Object%20Reference) (OtherBodyIndex :type Integer))
  (if (== (Utilities|GetClass OtherActor) "/Game/Blueprint/VirtualRealityBP/bpMotionController.bpMotionController_C")
    (Rendering|Material|SetMaterial (Variables|Default|GetStartLevel1) 0 "/Game/Meshes/Menu/Materials/unhighlightedBackground.unhighlightedBackground")
    (Rendering|Components|TextRender|SetTextRenderColor (Variables|Default|GetStartGameText) (Math|Conversions|ToColor(LinearColor) (Math|Color|MakeColor 0.0 0.0 0.0 255.0)))
    (Variables|Default|SetisTargetingStartLevel1 false)))

(event EventBeginPlay
  (bind _asmotion_controller_pawn (Utilities|Casting|CastToMotionControllerPawn (Pawn|GetControlledPawn (Game|GetPlayerController 0))))
  (Variables|Default|SetMotionControllerPawn _asmotion_controller_pawn))

(event Collision|EventActorBeginOverlap
  (params (OtherActor :type Actor%20Object%20Reference)))

(event EventTick
  (params (DeltaSeconds :type Float%20%28single-precision%29)))

(event Input|ActionEvents|InputActionGrabLeft
  (params (Key :type Key%20Structure))
  (:Pressed
    (if (Variables|Default|GetisTargetingStartLevel1)
      (Game|OpenLevel(byName) "Court1")
      (elif (Variables|Default|GetisTargetingLevels)
        _))))

(event Input|ActionEvents|InputActionGrabRight
  (params (Key :type Key%20Structure))
  (:Pressed
    (if (Variables|Default|GetisTargetingStartLevel1)
      (Game|OpenLevel(byName) "Court1")
      (elif (Variables|Default|GetisTargetingLevels)
        _))))

(fn ConstructionScript)