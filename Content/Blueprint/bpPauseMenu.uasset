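; VR pause menu actor with Main Menu and Resume buttons that respond to motion controller overlap.
; On BeginPlay it caches the player's MotionControllerPawn.
; When a BpMotionController begins or ends overlap with a button, it swaps that button's background material and text color for highlighting.
; The same events toggle the pawn's IsTargetingMenu or IsTargetingReturn flag; the menu itself performs neither action.
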(event OnComponentBeginOverlap(MainMenu)
  (params (OverlappedComponent :type Primitive%20Component%20Object%20Reference) (OtherActor :type Actor%20Object%20Reference) (OtherComp :type Primitive%20Component%20Object%20Reference) (OtherBodyIndex :type Integer) (bFromSweep :type Boolean) (SweepResult :type Hit%20Result%20Structure%20%28by%20ref%29))
  (if (== (Utilities|GetClass OtherActor) "/Game/Blueprint/VirtualRealityBP/bpMotionController.bpMotionController_C")
    (Rendering|Material|SetMaterial (Variables|Default|GetMainMenu) 0 "/Game/Meshes/Menu/Materials/highlightedBackground.highlightedBackground")
    (Rendering|Components|TextRender|SetTextRenderColor (Variables|Default|GetMainMenuText) (Math|Conversions|ToColor(LinearColor) (Math|Color|MakeColor 255.0 255.0 255.0 255.0)))
    (Variables|/Game/Blueprint/VirtualRealityBP/MotionControllerPawn.MotionControllerPawn_C|SetisTargetingMenu (Variables|Default|GetMotionControllerPawn) true)))

(event OnComponentEndOverlap(MainMenu)
  (params (OverlappedComponent :type Primitive%20Component%20Object%20Reference) (OtherActor :type Actor%20Object%20Reference) (OtherComp :type Primitive%20Component%20Object%20Reference) (OtherBodyIndex :type Integer))
  (if (== (Utilities|GetClass OtherActor) "/Game/Blueprint/VirtualRealityBP/bpMotionController.bpMotionController_C")
    (Rendering|Material|SetMaterial (Variables|Default|GetMainMenu) 0 "/Game/Meshes/Menu/Materials/unhighlightedBackground.unhighlightedBackground")
    (Rendering|Components|TextRender|SetTextRenderColor (Variables|Default|GetMainMenuText) (Math|Conversions|ToColor(LinearColor) (Math|Color|MakeColor 0.0 0.0 0.0 255.0)))
    (Variables|/Game/Blueprint/VirtualRealityBP/MotionControllerPawn.MotionControllerPawn_C|SetisTargetingMenu (Variables|Default|GetMotionControllerPawn) false)))

(event OnComponentBeginOverlap(Resume)
  (params (OverlappedComponent :type Primitive%20Component%20Object%20Reference) (OtherActor :type Actor%20Object%20Reference) (OtherComp :type Primitive%20Component%20Object%20Reference) (OtherBodyIndex :type Integer) (bFromSweep :type Boolean) (SweepResult :type Hit%20Result%20Structure%20%28by%20ref%29))
  (if (== (Utilities|GetClass OtherActor) "/Game/Blueprint/VirtualRealityBP/bpMotionController.bpMotionController_C")
    (Rendering|Material|SetMaterial (Variables|Default|GetResume) 0 "/Game/Meshes/Menu/Materials/highlightedBackground.highlightedBackground")
    (Rendering|Components|TextRender|SetTextRenderColor (Variables|Default|GetResumeText) (Math|Conversions|ToColor(LinearColor) (Math|Color|MakeColor 255.0 255.0 255.0 255.0)))
    (Variables|/Game/Blueprint/VirtualRealityBP/MotionControllerPawn.MotionControllerPawn_C|SetisTargetingReturn (Variables|Default|GetMotionControllerPawn) true)))

(event OnComponentEndOverlap(Resume)
  (params (OverlappedComponent :type Primitive%20Component%20Object%20Reference) (OtherActor :type Actor%20Object%20Reference) (OtherComp :type Primitive%20Component%20Object%20Reference) (OtherBodyIndex :type Integer))
  (if (== (Utilities|GetClass OtherActor) "/Game/Blueprint/VirtualRealityBP/bpMotionController.bpMotionController_C")
    (Rendering|Material|SetMaterial (Variables|Default|GetResume) 0 "/Game/Meshes/Menu/Materials/unhighlightedBackground.unhighlightedBackground")
    (Rendering|Components|TextRender|SetTextRenderColor (Variables|Default|GetResumeText) (Math|Conversions|ToColor(LinearColor) (Math|Color|MakeColor 0.0 0.0 0.0 255.0)))
    (Variables|/Game/Blueprint/VirtualRealityBP/MotionControllerPawn.MotionControllerPawn_C|SetisTargetingReturn (Variables|Default|GetMotionControllerPawn) false)))

(event EventBeginPlay
  (bind _asmotion_controller_pawn (Utilities|Casting|CastToMotionControllerPawn (Pawn|GetControlledPawn (Game|GetPlayerController 0))))
  (Variables|Default|SetMotionControllerPawn _asmotion_controller_pawn))

(event Collision|EventActorBeginOverlap
  (params (OtherActor :type Actor%20Object%20Reference)))

(event EventTick
  (params (DeltaSeconds :type Float%20%28single-precision%29)))

(fn ConstructionScript)